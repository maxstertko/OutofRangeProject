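; First-person player character with walk, sprint, crouch, jump and a toggled grappling hook fired by line trace at static world objects.
; Tick interpolates the Cable component's start to the hit point, then a DoOnce records the cable length on arrival.
; Holding PullGrapple launches the player toward the hook every frame.
; StopGrapple hides the cable and resets state, also triggering when distance exceeds the recorded length plus a margin.
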(event `self.ReceiveBeginPlay`
  (bind _cable (`self.Cable`))
  (bind _arms (`self.Arms`))
  (bind _returnvalue_location (`KismetMathLibrary.BreakTransform` (`SceneComponent.GetSocketTransform` _arms "HandRSocket" "RTS_Actor")))
  ;[1 1 1] Movement Start Parameters
  (set `CharacterMovementComponent.MaxWalkSpeed` (`self.WalkSpeed`) (`self.CharacterMovement`))
  ;[1 1 1] Cable Start Parameters
  (`SceneComponent.SetVisibility` _cable false false)
  (set `CableComponent.CableLength` 0.0 _cable)
  (set `CableComponent.CableWidth` 2.0 _cable)
  (`SceneComponent.K2_SetWorldLocation` _cable (`SceneComponent.GetSocketLocation` _arms "HandRSocket") false false)
  (bind _output_get (set `self.StartEndLocation` _returnvalue_location))
  (set `CableComponent.EndLocation` _output_get _cable))

(event `InputAction|Jump`
  (params (Key :type "Key Structure"))
  ;[1 1 1] Basic Movement
  (:`Pressed`
    (`self.Jump`)))

(event `InputAxis|Turn`
  (params (AxisValue :type "Float (single-precision)"))
  ;[1 1 1] Aim
  (`self.AddControllerYawInput` AxisValue))

(event `InputAction|Fire`
  (params (Key :type "Key Structure"))
  (bind _camera (`self.Camera`))
  (bind _returnvalue (`SceneComponent.K2_GetComponentLocation` _camera))
  (:`Pressed`
    (`/Engine/EditorBlueprintResources/StandardMacros.FlipFlop`
      (:`A`
        (bind _outhit (`KismetSystemLibrary.LineTraceSingleForObjects` :`Start` _returnvalue :`End` (+ _returnvalue (* (`SceneComponent.GetForwardVector` _camera) (`self.GrappleDistance`))) :`ObjectTypes` (`|MakeArray` "ObjectTypeQuery1" :!type "EObjectTypeQuery Enum") :`DrawDebugType` "ForDuration"))
        (if (`GameplayStatics.BreakHitResult` _outhit)
          (set `self.Hooked` true)
          (set `self.HookLocation` (`.Location` (`GameplayStatics.BreakHitResult` _outhit)))
          (else
            (`self.StopGrapple`))))
      (:`B`
        (`self.StopGrapple`)
        (set `CableComponent.EndLocation` (`self.StartEndLocation`) (`self.Cable`))))))

(event `InputAxis|LookUp`
  (params (AxisValue :type "Float (single-precision)"))
  ;[1 1 1] Aim
  (`self.AddControllerPitchInput` AxisValue))

(event `InputAxis|MoveForward`
  (params (AxisValue :type "Float (single-precision)"))
  ;[1 1 1] Basic Movement
  (`self.AddMovementInput` (`self.GetActorForwardVector`) AxisValue))

(event `InputAxis|MoveRight`
  (params (AxisValue :type "Float (single-precision)"))
  ;[1 1 1] Basic Movement
  (`self.AddMovementInput` (`self.GetActorRightVector`) AxisValue))

(event `self.ReceiveTick`
  (params (DeltaSeconds :type "Float (single-precision)"))
  (bind _cable (`self.Cable`))
  (bind _cable_2 (`self.Cable`))
  (if (`self.Hooked`)
    (`self.PullOnPress`)
    (if (`self.HookMoveFinished`)
      (`|ExecutionSequence`
        (:`then_0`
          ;[1 1 1] Move Start Position of Hook
          (`SceneComponent.K2_SetWorldLocationAndRotation` _cable (`KismetMathLibrary.VInterpTo` (`SceneComponent.K2_GetComponentLocation` _cable) (`self.HookLocation`) (`GameplayStatics.GetWorldDeltaSeconds`) 250.0) (`KismetMathLibrary.FindLookAtRotation` (`self.K2_GetActorLocation`) (`self.HookLocation`)) false false)
          ;[1 1 1] Set new cable length
          (`/Engine/EditorBlueprintResources/StandardMacros.DoOnce` false :!label _label
            (:`Completed`
              (bind _output_get (set `CableComponent.CableLength` (`KismetMathLibrary.VSize` (- (`self.K2_GetActorLocation`) (`self.HookLocation`))) _cable_2))
              (bind _output_get_2 (set `self.NewCableLength` _output_get))
              (`SceneComponent.K2_SetWorldLocation` _cable_2 (`SceneComponent.GetSocketLocation` (`self.Arms`) "HandRSocket") false false)
              (set `CableComponent.EndLocation` (`self.StartEndLocation`) _cable_2)
              (`KismetSystemLibrary.PrintString` (`KismetStringLibrary.Conv_DoubleToString` _output_get_2)))))
        (:`then_1`
          ;[1 1 1] Breaks cable when tense but switch to hold player position
          (if (>= (`KismetMathLibrary.VSize` (- (`self.K2_GetActorLocation`) (`self.HookLocation`))) (+ (`self.NewCableLength`) 400.0))
            (`self.StopGrapple`))))
      (else
        (bind _reachedlocation (`self.MoveCable`))
        (set `self.HookMoveFinished` _reachedlocation)))))

(event `InputAction|Sprint`
  (params (Key :type "Key Structure"))
  (bind _charactermovement (`self.CharacterMovement`))
  ;[1 1 1] Basic Movement
  (:`Pressed`
    (set `CharacterMovementComponent.MaxWalkSpeed` (`self.SprintSpeed`) _charactermovement))
  (:`Released`
    (set `CharacterMovementComponent.MaxWalkSpeed` (`self.WalkSpeed`) _charactermovement)))

(event `Key|C`
  (params (Key :type "Key Structure"))
  (bind _charactermovement (`self.CharacterMovement`))
  (:`Pressed`
    (`self.Crouch`)
    (set `CharacterMovementComponent.MaxWalkSpeedCrouched` (`self.SprintSpeed`) _charactermovement)
    (`KismetSystemLibrary.PrintString` "Hello" (`self.bIsCrouched`)))
  (:`Released`
    (`self.UnCrouch`)
    (set `CharacterMovementComponent.MaxWalkSpeedCrouched` (`self.WalkSpeed`) _charactermovement)))

(event `StopGrapple`
  (bind _cable (`self.Cable`))
  ;[1 1 1] Stop Grapple
  (set `self.Hooked` false)
  (set `self.HookMoveFinished` false)
  (`SceneComponent.SetVisibility` _cable false false)
  (`SceneComponent.K2_SetWorldLocation` _cable (`self.K2_GetActorLocation`) false false)
  (goto _label :!via `Reset`))

(event `InputAction|PullGrapple`
  (params (Key :type "Key Structure"))
  (:`Pressed`
    (set `self.isPulling` true))
  (:`Released`
    (set `self.isPulling` false)))

(event `PullOnPress`
  (if (`self.isPulling`)
    (`self.MovePlayer`)
    (set `CableComponent.CableLength` (`KismetMathLibrary.VSize` (- (`self.K2_GetActorLocation`) (`self.HookLocation`))) (`self.Cable`))))

(fn `MoveCable`
  (returns (ReachedLocation :type Boolean))
  (bind _cable (`self.Cable`))
  (bind _hooklocation (`self.HookLocation`))
  (bind _returnvalue (`SceneComponent.K2_GetComponentLocation` _cable))
  (`SceneComponent.SetVisibility` _cable true false)
  (if (<= (`KismetMathLibrary.VSize` (- _returnvalue _hooklocation)) 100.0)
    (return true)
    (else
      (`SceneComponent.K2_SetWorldLocation` _cable (`KismetMathLibrary.VInterpTo` _returnvalue _hooklocation (`GameplayStatics.GetWorldDeltaSeconds`) 10.0) false false)
      (return false))))

(fn `MovePlayer`
  (`self.LaunchCharacter` (* (- (`self.HookLocation`) (`self.K2_GetActorLocation` (`GameplayStatics.GetPlayerPawn` 0))) (* (`GameplayStatics.GetWorldDeltaSeconds`) 75.0)) true true))

(fn `UserConstructionScript`)