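; First-person-style player character with walking, mouse look, jumping, sprinting and the start of a grappling hook.
; Fire line-traces from the camera against world objects up to the grapple distance, turns the actor toward a hit and stores the hooked state and location.
; The Grapple cable is configured and hidden at BeginPlay; this graph contains no pull movement or cable update.
; Shift swaps max walk speed between sprint and the cached default.
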(event `self.ReceiveBeginPlay`
  (bind _grapple (`self.Grapple`))
  (set `self.WalkSpeed` (`CharacterMovementComponent.MaxWalkSpeed` (`self.CharacterMovement`)))
  (`SceneComponent.SetVisibility` _grapple false false)
  (set `CableComponent.CableLength` 0.0 _grapple)
  (set `CableComponent.CableWidth` 2.0 _grapple)
  (set `CableComponent.EndLocation` (120.0 10.0 60.0) _grapple))

(event `InputAction|Fire`
  (params (Key :type "Key Structure"))
  (bind _camera (`self.Camera`))
  (bind _returnvalue (`SceneComponent.K2_GetComponentLocation` _camera))
  (:`Pressed`
    (bind _outhit (`KismetSystemLibrary.LineTraceSingleForObjects` :`Start` _returnvalue :`End` (+ _returnvalue (* (`SceneComponent.GetForwardVector` _camera) (`self.GrappleDistance`))) :`ObjectTypes` (`|MakeArray` "ObjectTypeQuery1" "ObjectTypeQuery2" :!type "EObjectTypeQuery Enum") :`DrawDebugType` "ForDuration"))
    (if (`GameplayStatics.BreakHitResult` _outhit)
      (bind (_returnvalue_roll _returnvalue_pitch _returnvalue_yaw) (`KismetMathLibrary.BreakRotator` (`KismetMathLibrary.FindLookAtRotation` (`self.K2_GetActorLocation`) (`.Location` (`GameplayStatics.BreakHitResult` _outhit)))))
      (`self.K2_SetActorRotation` (`KismetMathLibrary.MakeRotator` 0.0 _returnvalue_pitch _returnvalue_yaw))
      (set `self.isHooked` true)
      (set `self.HookLocation` (`.Location` (`GameplayStatics.BreakHitResult` _outhit))))))

(event `InputAxis|MoveForward`
  (params (AxisValue :type "Float (single-precision)"))
  ;[1 1 1] Basic movement and Aiming
  (`self.AddMovementInput` (`self.GetActorForwardVector`) AxisValue))

(event `InputAxis|LookUp`
  (params (AxisValue :type "Float (single-precision)"))
  ;[1 1 1] Basic movement and Aiming
  (`self.AddControllerPitchInput` AxisValue))

(event `InputAxis|MoveRight`
  (params (AxisValue :type "Float (single-precision)"))
  ;[1 1 1] Basic movement and Aiming
  (`self.AddMovementInput` (`self.GetActorRightVector`) AxisValue))

(event `InputAxis|Turn`
  (params (AxisValue :type "Float (single-precision)"))
  ;[1 1 1] Basic movement and Aiming
  (`self.AddControllerYawInput` AxisValue))

(event `Key|LeftShift`
  (params (Key :type "Key Structure"))
  (bind _charactermovement (`self.CharacterMovement`))
  ;[1 1 1] Jumping and Sprinting
  (:`Pressed`
    (set `CharacterMovementComponent.MaxWalkSpeed` (`self.SprintSpeed`) _charactermovement))
  (:`Released`
    (set `CharacterMovementComponent.MaxWalkSpeed` (`self.WalkSpeed`) _charactermovement)))

(event `InputAction|Jump`
  (params (Key :type "Key Structure"))
  ;[1 1 1] Jumping and Sprinting
  (:`Pressed`
    (`self.Jump`)))

(fn `UserConstructionScript`)